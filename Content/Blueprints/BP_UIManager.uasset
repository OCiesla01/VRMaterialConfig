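; BP_UIManager links a VR material selection UI to the material manager, model stand and save-to-file button.
; PopulateMaterialSelectorPanel reads a materials data table and adds a WBP_MaterialBtn per row to its category's wrap box, binding each button's press event.
; ApplyMaterial assigns the material through BP_MaterialManager, shows its name on the stand and passes name and link to the save button.
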(event `self.ReceiveBeginPlay`
  (bind _returnvalue (`GameplayStatics.GetActorOfClass` "/Game/VRTemplate/Blueprints/VRPawn.VRPawn_C"))
  (set `self.VRPawnRef` _returnvalue)
  (bind _returnvalue_2 (`GameplayStatics.GetActorOfClass` "/Game/Blueprints/BP_MaterialManager.BP_MaterialManager_C"))
  (set `self.MaterialManagerRef` _returnvalue_2)
  (bind _returnvalue_3 (`GameplayStatics.GetActorOfClass` "/Game/Blueprints/BP_ModelStand.BP_ModelStand_C"))
  (set `self.ModelStandRef` _returnvalue_3)
  (bind _returnvalue_4 (`GameplayStatics.GetActorOfClass` "/Game/Blueprints/Buttons/BP_ButtonSaveToFile.BP_ButtonSaveToFile_C"))
  (set `self.ButtonSaveToFileRef` _returnvalue_4))

(event `ApplyMaterial`
  (params (Material :type "MaterialInstance Object Reference") (Name :type Text) (Link :type Text))
  (bind _buttonsavetofileref (`self.ButtonSaveToFileRef`))
  (`/Game/Blueprints/BP_MaterialManager.AssignMaterial` (`self.MaterialManagerRef`) Material)
  (`self.SetDisplayName` Name)
  (set `/Game/Blueprints/Buttons/BP_ButtonSaveToFile.Name` Name _buttonsavetofileref)
  (set `/Game/Blueprints/Buttons/BP_ButtonSaveToFile.Link` Link _buttonsavetofileref))

(fn `CreateAndSetupIndividualTextureUI`
  (params (WrapBoxParent :type "WrapBox Object Reference") (TextureBaseImage :type "Texture Object Reference") (Material :type "MaterialInstance Object Reference") (Name :type Text) (Link :type Text))
  (bind _returnvalue (`|CreateWidget` "/Game/UI/WBP_MaterialBtn.WBP_MaterialBtn_C"))
  (`PanelWidget.AddChild` WrapBoxParent _returnvalue)
  (`self.SetTextureBaseImage` _returnvalue TextureBaseImage)
  (`/Game/UI/WBP_MaterialBtn.SetDynamicMaterial` _returnvalue Material)
  (`/Game/UI/WBP_MaterialBtn.SetName` _returnvalue Name)
  (`/Game/UI/WBP_MaterialBtn.SetLink` _returnvalue Link)
  (add `/Game/UI/WBP_MaterialBtn.OnMaterialPressed` _returnvalue (`|CreateDelegate` :!event `ApplyMaterial`)))

(fn `PopulateMaterialSelectorPanel`
  (params (WrapBoxParent :type "Map of String to WrapBox Object Reference"))
  (bind _outrownames (`DataTableFunctionLibrary.GetDataTableRowNames` (`self.MaterialsDT`)))
  (for _array_element _outrownames
    (bind _returnvalue (`|GetDataTableRow` (`self.MaterialsDT`) _array_element)
      (:`then`
        (bind (_category _basetexture _material _name _link) (break `/Game/Data/S_Material` _returnvalue))
        (set `self.TempBaseTexture` _basetexture)
        (set `self.TempMaterial` _material)
        (set `self.TempWrapBox` (`BlueprintMapLibrary.Map_Find` WrapBoxParent (`|GetEnumeratorNameAsString` _category)))
        (set `self.TempName` _name)
        (set `self.TempLink` _link)
        (switch `/Game/Data/E_MaterialCategory` _category
          (:`NewEnumerator0`
            (`self.CreateAndSetupIndividualTextureUI` (`self.TempWrapBox`) (`self.TempBaseTexture`) (`self.TempMaterial`) (`self.TempName`) (`self.TempLink`)))
          (:`NewEnumerator4`
            (`self.CreateAndSetupIndividualTextureUI` (`self.TempWrapBox`) (`self.TempBaseTexture`) (`self.TempMaterial`) (`self.TempName`) (`self.TempLink`)))
          (:`NewEnumerator2`
            (`self.CreateAndSetupIndividualTextureUI` (`self.TempWrapBox`) (`self.TempBaseTexture`) (`self.TempMaterial`) (`self.TempName`) (`self.TempLink`)))
          (:`NewEnumerator1`
            (`self.CreateAndSetupIndividualTextureUI` (`self.TempWrapBox`) (`self.TempBaseTexture`) (`self.TempMaterial`) (`self.TempName`) (`self.TempLink`)))
          (:`NewEnumerator3`
            (`self.CreateAndSetupIndividualTextureUI` (`self.TempWrapBox`) (`self.TempBaseTexture`) (`self.TempMaterial`) (`self.TempName`) (`self.TempLink`))))))))

(fn `SetDisplayName`
  (params (`Material Name` :type Text))
  (`TextRenderComponent.K2_SetText` (`/Game/Blueprints/BP_ModelStand.MaterialNameText` (`self.ModelStandRef`)) `Material Name`))

(fn `SetTextureBaseImage`
  (params (MaterialBtn :type "/Game/UI/WBP_MaterialBtn Object Reference") (TextureBaseImage :type "Texture Object Reference"))
  (`Image.SetBrush` (`/Game/UI/WBP_MaterialBtn.Image` MaterialBtn) (make `SlateBrush` (struct :`SpecifiedColor` (struct :`R` 1.0 :`G` 1.0 :`B` 1.0 :`A` 1.0) :`ColorUseRule` "UseColor_Specified") "Image" "NoTile" "NoMirror" (struct :`X` 32.0 :`Y` 32.0) (struct) TextureBaseImage)))

(fn `UserConstructionScript`)