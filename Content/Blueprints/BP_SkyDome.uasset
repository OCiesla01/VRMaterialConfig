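; BP_SkyDome is a sky dome actor that aims the level's directional light based on what overlaps its trigger.
; On BeginPlay it caches the first DirectionalLight actor it finds.
; When a component begins overlapping Trigger, the light is rotated to face along the direction from that component toward CenterPoint, as if shining from it.
; The rotation is set only on overlap begin, not updated continuously.
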(event `self.ReceiveBeginPlay`
  (bind _returnvalue (`GameplayStatics.GetActorOfClass` "/Script/Engine.DirectionalLight"))
  (set `self.DirectLightRef` _returnvalue))

(event `self.Trigger.OnComponentBeginOverlap`
  (params (OverlappedComponent :type "PrimitiveComponent Object Reference") (OtherActor :type "Actor Object Reference") (OtherComp :type "PrimitiveComponent Object Reference") (OtherBodyIndex :type Integer) (bFromSweep :type Boolean) (SweepResult :type "HitResult Structure (by ref)"))
  (`self.K2_SetActorRotation` (`self.DirectLightRef`) (`KismetMathLibrary.MakeRotFromX` (`KismetMathLibrary.NegateVector` (`KismetMathLibrary.Normal` (- (`SceneComponent.K2_GetComponentLocation` OtherComp) (`SceneComponent.K2_GetComponentLocation` (`self.CenterPoint`)))))) false))

(fn `UserConstructionScript`)