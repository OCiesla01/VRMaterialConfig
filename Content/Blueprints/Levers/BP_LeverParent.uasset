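; Base VR lever actor that a motion controller can grab and tilt in either direction around a spring-back center.
; While held, a fast looping timer runs UpdateRotation, converting the controller's offset from the grab component into clamped pitch on the Scene component.
; Beyond a small dead zone, each update fires OnRotationNegative or OnRotationPositive.
; On release, the timer stops and a timeline lerps pitch back to zero.
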(event `self.GrabComponent.OnGrabbed`
  (params (MotionController :type "MotionControllerComponent Object Reference"))
  (set `self.MotionControllerRef` MotionController)
  (bind _returnvalue (`KismetSystemLibrary.K2_SetTimer` null "UpdateRotation" 0.01 true))
  (set `self.Timer` _returnvalue))

(event `self.GrabComponent.OnDropped`
  (bind (_relativerotation_roll _relativerotation_pitch) (`KismetMathLibrary.BreakRotator` (`SceneComponent.RelativeRotation` (`self.Scene`))))
  (`KismetSystemLibrary.K2_ClearAndInvalidateTimerHandle` (`self.Timer`))
  (set `self.MotionControllerRef` null)
  (bind (_direction _alpha) (`Timeline|T_ResetRotation` :!via `PlayFromStart`)
    (:`Update`
      (`SceneComponent.K2_SetRelativeRotation` (`self.Scene`) (`KismetMathLibrary.MakeRotator` 0.0 (`KismetMathLibrary.Lerp` _relativerotation_pitch 0.0 _alpha)) false false))))

(fn `UpdateRotation`
  (bind _grabcomponent (`self.GrabComponent`))
  (bind (_relativerotation_roll _relativerotation_pitch _relativerotation_yaw) (`KismetMathLibrary.BreakRotator` (`SceneComponent.RelativeRotation` (`self.Scene`))))
  (bind _returnvalue_location (`KismetMathLibrary.BreakTransform` (`KismetMathLibrary.MakeRelativeTransform` (`SceneComponent.K2_GetComponentToWorld` (`self.MotionControllerRef`)) (`SceneComponent.K2_GetComponentToWorld` _grabcomponent))))
  (bind _returnvalue_x (`KismetMathLibrary.BreakVector` (- (`SceneComponent.RelativeLocation` _grabcomponent) _returnvalue_location)))
  (bind _returnvalue (`KismetMathLibrary.FClamp` (+ _returnvalue_x _relativerotation_pitch) -30.0 30.0))
  (`SceneComponent.K2_SetRelativeRotation` (`self.Scene`) (`KismetMathLibrary.MakeRotator` _relativerotation_roll _returnvalue _relativerotation_yaw) false false)
  (if (< _returnvalue -5.0)
    (`self.OnRotationNegative`)
    (elif (> _returnvalue 5.0)
      (`self.OnRotationPositive`))))

(fn `UserConstructionScript`)