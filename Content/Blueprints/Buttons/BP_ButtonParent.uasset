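; BP_ButtonParent is a pressure button, named as a parent class, that fires when something overlaps its Trigger.
; Overlap begin calls OnPressed, plays a sound and runs a timeline that slightly squashes ButtonMesh's Z scale, relative to StaticMesh's scale.
; Overlap end calls OnUnpressed and reverses the timeline.
; An IsOverlapped flag blocks repeat presses, but overlaps are neither filtered nor counted, so any exit releases it.
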(event `self.Trigger.OnComponentBeginOverlap`
  (params (OverlappedComponent :type "PrimitiveComponent Object Reference") (OtherActor :type "Actor Object Reference") (OtherComp :type "PrimitiveComponent Object Reference") (OtherBodyIndex :type Integer) (bFromSweep :type Boolean) (SweepResult :type "HitResult Structure (by ref)"))
  (bind (_returnvalue_x _returnvalue_y _returnvalue_z) (`KismetMathLibrary.BreakVector` (`SceneComponent.K2_GetComponentScale` (`self.StaticMesh`))))
  (if (not (`self.bIsOverlapped`))
    (set `self.bIsOverlapped` true)
    (`self.OnPressed`)
    (`GameplayStatics.PlaySoundAtLocation` "/Game/Audio/button_pressed.button_pressed" (`SceneComponent.K2_GetComponentLocation` (`self.StaticMesh`)) (struct) 1.0 1.0 0.0 null null null null)
    (bind (_direction _scale) (`Timeline|T_ButtonZScale` :!via `PlayFromStart` :!label _label)
      (:`Update`
        (`SceneComponent.SetWorldScale3D` (`self.ButtonMesh`) (`KismetMathLibrary.MakeVector` _returnvalue_x _returnvalue_y (`KismetMathLibrary.Lerp` _returnvalue_z (- _returnvalue_z 0.03) _scale)))))))

(event `self.Trigger.OnComponentEndOverlap`
  (params (OverlappedComponent :type "PrimitiveComponent Object Reference") (OtherActor :type "Actor Object Reference") (OtherComp :type "PrimitiveComponent Object Reference") (OtherBodyIndex :type Integer))
  (if (`self.bIsOverlapped`)
    (set `self.bIsOverlapped` false)
    (`self.OnUnpressed`)
    (goto _label :!via `ReverseFromEnd`)))

(fn `UserConstructionScript`)