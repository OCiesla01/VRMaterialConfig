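; BP_ResetModel is a button Blueprint that resets the main model's static mesh transform when its Trigger component is overlapped.
; At BeginPlay it finds the BP_MainModel actor and caches its mesh's world transform as the baseline.
; While IsFirstReset is set, an overlap restores the full baseline and clears the flag.
; Otherwise it restores only location and rotation and forces a fixed half scale.
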(event `self.ReceiveBeginPlay`
  (bind _returnvalue (`GameplayStatics.GetActorOfClass` "/Game/Blueprints/BP_MainModel.BP_MainModel_C"))
  (bind _output_get (set `self.MainModelRef` _returnvalue))
  (set `self.BaseTransform` (`SceneComponent.K2_GetComponentToWorld` (`/Game/Blueprints/BP_MainModel.StaticMesh` _output_get))))

(event `self.Trigger.OnComponentBeginOverlap`
  (params (OverlappedComponent :type "PrimitiveComponent Object Reference") (OtherActor :type "Actor Object Reference") (OtherComp :type "PrimitiveComponent Object Reference") (OtherBodyIndex :type Integer) (bFromSweep :type Boolean) (SweepResult :type "HitResult Structure (by ref)"))
  (bind (_basetransform_location _basetransform_rotation) (`KismetMathLibrary.BreakTransform` (`self.BaseTransform`)))
  (bind _staticmesh (`/Game/Blueprints/BP_MainModel.StaticMesh` (`self.MainModelRef`)))
  (if (`self.bIsFirstReset`)
    (`SceneComponent.K2_SetWorldTransform` _staticmesh (`self.BaseTransform`) false false)
    (set `self.bIsFirstReset` false)
    (else
      (`SceneComponent.K2_SetWorldTransform` _staticmesh (`KismetMathLibrary.MakeTransform` _basetransform_location _basetransform_rotation (0.5 0.5 0.5)) false false))))

(fn `UserConstructionScript`
  (`parent.UserConstructionScript`))