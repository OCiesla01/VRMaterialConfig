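; BP_ButtonShowPanel is a button actor that shows and hides the material management panel.
; On BeginPlay, after calling its parent, it caches a reference to the BP_MaterialManagePanel actor found in the level.
; Each begin overlap on its Trigger component, with no filter on the overlapping actor, flips the panel's IsVisible flag and sets MainSM visibility to match, propagating to child components.
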(event `self.ReceiveBeginPlay`
  (`parent.ReceiveBeginPlay`)
  (bind _returnvalue (`GameplayStatics.GetActorOfClass` "/Game/Blueprints/BP_MaterialManagePanel.BP_MaterialManagePanel_C"))
  (set `self.MaterialManagePanelRef` _returnvalue))

(event `self.Trigger.OnComponentBeginOverlap`
  (params (OverlappedComponent :type "PrimitiveComponent Object Reference") (OtherActor :type "Actor Object Reference") (OtherComp :type "PrimitiveComponent Object Reference") (OtherBodyIndex :type Integer) (bFromSweep :type Boolean) (SweepResult :type "HitResult Structure (by ref)"))
  (bind _materialmanagepanelref (`self.MaterialManagePanelRef`))
  (bind _mainsm (`/Game/Blueprints/BP_MaterialManagePanel.MainSM` (`self.MaterialManagePanelRef`)))
  (if (`/Game/Blueprints/BP_MaterialManagePanel.bIsVisible` (`self.MaterialManagePanelRef`))
    (`SceneComponent.SetVisibility` _mainsm false true)
    (set `/Game/Blueprints/BP_MaterialManagePanel.bIsVisible` false _materialmanagepanelref)
    (else
      (`SceneComponent.SetVisibility` _mainsm true true)
      (set `/Game/Blueprints/BP_MaterialManagePanel.bIsVisible` true _materialmanagepanelref))))

(fn `UserConstructionScript`
  (`parent.UserConstructionScript`))