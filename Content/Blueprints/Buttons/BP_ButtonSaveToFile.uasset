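; Trigger button that saves the current material's tuning settings to a text file in the project's Saved directory when something overlaps it.
; On BeginPlay it finds BP_MaterialManager and sets that manager's save path.
; On overlap it reads UV tiling/offset and surface scalar parameters from the manager's TempMaterial, formats them with a name and link, and writes them to a .txt named after Name.
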(event `self.ReceiveBeginPlay`
  (bind _returnvalue (`GameplayStatics.GetActorOfClass` "/Game/Blueprints/BP_MaterialManager.BP_MaterialManager_C"))
  (bind _output_get (set `self.MaterialManagerRef` _returnvalue))
  (set `/Game/Blueprints/BP_MaterialManager.SaveFilePath` (`KismetSystemLibrary.GetProjectSavedDirectory`) _output_get))

(event `self.Trigger.OnComponentBeginOverlap`
  (params (OverlappedComponent :type "PrimitiveComponent Object Reference") (OtherActor :type "Actor Object Reference") (OtherComp :type "PrimitiveComponent Object Reference") (OtherBodyIndex :type Integer) (bFromSweep :type Boolean) (SweepResult :type "HitResult Structure (by ref)"))
  (`self.SaveFile` (`self.Name`)))

(fn `CreateText`
  (returns (Text :type String))
  (bind (_u_tiling _v_tiling _u_offset _v_offset _brightness _saturation _contrast _specular _normal _ao _rmin _rmax) (`self.GetMaterialParameterValues`))
  (return (`KismetTextLibrary.Conv_TextToString` (`|FormatText` "{name} - {link} \n[Global Settings] \nU Tiling: {utiling} \nV Tiling: {vtiling} \nU Offset: {uoffset} \nV Offset: {voffset} \n \n[Diffuse] \nBrightness: {brightness} \nSaturation: {saturation} \nContrast: {contrast} \n \n[Specular] \nValue: {specular} \n \n[Normal] \nStrength: {normal} \n \n[AO] \nStrength: {ao} \n \n[Roughness] \nMin: {rmin} \nMax: {rmax}" (`self.Name`) (`self.Link`) _u_tiling _v_tiling _u_offset _v_offset _brightness _saturation _contrast _specular _normal _ao _rmin _rmax))))

(fn `GetMaterialParameterValues`
  (returns (`U Tiling` :type "Float (double-precision)") (`V Tiling` :type "Float (double-precision)") (`U Offset` :type "Float (double-precision)") (`V Offset` :type "Float (double-precision)") (Brightness :type "Float (double-precision)") (Saturation :type "Float (double-precision)") (Contrast :type "Float (double-precision)") (Specular :type "Float (double-precision)") (Normal :type "Float (double-precision)") (AO :type "Float (double-precision)") (RMin :type "Float (double-precision)") (RMax :type "Float (double-precision)"))
  (bind _tempmaterial (`/Game/Blueprints/BP_MaterialManager.TempMaterial` (`self.MaterialManagerRef`)))
  (bind _returnvalue (`MaterialInstanceDynamic.K2_GetVectorParameterValue` (`/Game/Blueprints/BP_MaterialManager.TempMaterial` (`self.MaterialManagerRef`)) "Advanced UV Tiling & Offset"))
  (bind _returnvalue_2 (`MaterialInstanceDynamic.K2_GetScalarParameterValue` _tempmaterial "D_Brightness"))
  (bind _returnvalue_3 (`MaterialInstanceDynamic.K2_GetScalarParameterValue` _tempmaterial "D_Saturation"))
  (bind _returnvalue_4 (`MaterialInstanceDynamic.K2_GetScalarParameterValue` _tempmaterial "D_Contrast"))
  (bind _returnvalue_5 (`MaterialInstanceDynamic.K2_GetScalarParameterValue` _tempmaterial "S_Specular Override"))
  (bind _returnvalue_6 (`MaterialInstanceDynamic.K2_GetScalarParameterValue` _tempmaterial "N_Strength"))
  (bind _returnvalue_7 (`MaterialInstanceDynamic.K2_GetScalarParameterValue` _tempmaterial "AO_Strength"))
  (bind _returnvalue_8 (`MaterialInstanceDynamic.K2_GetScalarParameterValue` _tempmaterial "R_MinRoughness"))
  (bind _returnvalue_9 (`MaterialInstanceDynamic.K2_GetScalarParameterValue` _tempmaterial "R_MaxRoughness"))
  (return (break `LinearColor` _returnvalue) (`.G` (break `LinearColor` _returnvalue)) (`.B` (break `LinearColor` _returnvalue)) (`.A` (break `LinearColor` _returnvalue)) _returnvalue_2 _returnvalue_3 _returnvalue_4 _returnvalue_5 _returnvalue_6 _returnvalue_7 _returnvalue_8 _returnvalue_9))

(fn `SaveFile`
  (params (Name :type Text))
  (if true
    (bind _text (`self.CreateText`))
    (`FileSDKBPLibrary.WriteStringToFile` (`KismetTextLibrary.Conv_TextToString` (`|FormatText` "{path}{name}.txt" (`/Game/Blueprints/BP_MaterialManager.SaveFilePath` (`self.MaterialManagerRef`)) Name)) _text)))

(fn `UserConstructionScript`
  (`parent.UserConstructionScript`))